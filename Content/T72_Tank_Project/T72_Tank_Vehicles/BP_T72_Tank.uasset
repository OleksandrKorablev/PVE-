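; Player-controlled T-72 tank pawn on Chaos wheeled vehicle movement, with throttle, brake and yaw steering input.
; Axis inputs accumulate clamped Gun and Turret angles, while mouse input rotates the camera and the wheel adjusts spring arm length.
; Left click plays a timeline driving recoil, muzzle effect and boom, gated by a DoOnce reset after a delay.
; Each tick, one wheel's angular velocity feeds a material scalar to animate the tracks.
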(event Custom|Track%20Animation
  ;[1 0 0.4798] Анімація гуслі
  (Rendering|Material|SetScalarParameterValueonMaterials (Variables|Character|GetMesh) "OffsetV" (Class|ChaosVehicleWheel|GetRotationAngularVelocity (Utilities|Array|Get(acopy) (Variables|/Script/ChaosVehicles.ChaosWheeledVehicleMovementComponent|GetWheels (Variables|Default|GetChaosWheeledVehicleMovement)) 4))))

(event EventTick
  (params (DeltaSeconds :type Float%20%28single-precision%29))
  ;[0.1925 0.1952 1] Event Tick
  (CallFunction|TrackAnimation))

(event Input|AxisEvents|InputAxisTurret
  (params (AxisValue :type Float%20%28single-precision%29))
  ;[1 0 0.4798] Башта
  (Variables|Default|SetTurret (Math|Float|Clamp(Float) (+ (Variables|Default|GetTurret) AxisValue) -1.8e+02 1.8e+02)))

(event Input|AxisEvents|InputAxisGun
  (params (AxisValue :type Float%20%28single-precision%29))
  ;[1 0 0.4798] Ствол
  (Variables|Default|SetGun (Math|Float|Clamp(Float) (+ (Variables|Default|GetGun) AxisValue) 0.0 25.0)))

(event Input|AxisEvents|InputAxisCameraControlerX
  (params (AxisValue :type Float%20%28single-precision%29))
  ;[1 0 0.4798] Вільний погляд
  (Pawn|Input|AddControllerYawInput AxisValue))

(event Input|AxisEvents|InputAxisCameraControlerY
  (params (AxisValue :type Float%20%28single-precision%29))
  ;[1 0 0.4798] Вільний погляд
  (Pawn|Input|AddControllerPitchInput AxisValue))

(event Input|AxisEvents|InputAxisMoveForward
  (params (AxisValue :type Float%20%28single-precision%29))
  (bind _chaoswheeledvehiclemovement (Variables|Default|GetChaosWheeledVehicleMovement))
  ;[1 0 0.4798] Рух танка
  (Class|ChaosVehicleMovementComponent|SetThrottleInput _chaoswheeledvehiclemovement AxisValue)
  (Class|ChaosVehicleMovementComponent|SetBrakeInput _chaoswheeledvehiclemovement (* AxisValue -1.0)))

(event Input|AxisEvents|InputAxisMoveRight
  (params (AxisValue :type Float%20%28single-precision%29))
  (bind _chaoswheeledvehiclemovement (Variables|Default|GetChaosWheeledVehicleMovement))
  ;[1 0 0.4798] Рух танка
  (Class|ChaosVehicleMovementComponent|SetYawInput _chaoswheeledvehiclemovement AxisValue)
  (Class|ChaosVehicleMovementComponent|SetBrakeInput _chaoswheeledvehiclemovement (* AxisValue -1.0)))

(event Input|MouseEvents|MouseX
  (params (AxisValue :type Float%20%28single-precision%29))
  ;[1 1 1] Mouse View
  ;;[1 1 1] Миша вліво/вправо
  (Transformation|AddWorldRotation (Variables|Default|GetSpringArm) (Math|Rotator|MakeRotator 0.0 0.0 AxisValue) false false))

(event Input|MouseEvents|MouseY
  (params (AxisValue :type Float%20%28single-precision%29))
  ;[1 1 1] Mouse View
  ;;[1 1 1] Миша вліво/вправо
  (Transformation|AddLocalRotation (Variables|Default|GetSpringArm) (Math|Rotator|MakeRotator 0.0 AxisValue 0.0) false false))

(event Input|MouseEvents|LeftMouseButton
  (params (Key :type Key%20Structure :default "None"))
  ;[1 0 0.4798] Вогонь
  (:Pressed
    (Utilities|FlowControl|DoOnce false :!label _label
      (:Completed
        (bind _recoil (Timeline|maingunfire PlayFromStart)
          (:Update
            (Variables|Default|Setrecoil (Math|Float|Lerp -5e+01 0.0 _recoil)))
          (:muzzle
            (Components|Activation|Activate (Variables|Default|Getmuzzle) true))
          (:audioexplosion
            (Components|Activation|Activate (Variables|Default|Getboom) true)))
        (Utilities|FlowControl|Delay 1.3)
        (goto _label Reset)))))

(event Input|MouseEvents|MouseWheelDown
  (params (Key :type Key%20Structure :default "None"))
  (bind _springarm (Variables|Default|GetSpringArm))
  ;[1 1 1] Mouse View
  ;;[1 1 1] Збільшення коліщатка дальності камери
  (:Pressed
    (Variables|/Script/Engine.SpringArmComponent|SetTargetArmLength _springarm (Math|Float|Max(Float) (+ (Variables|/Script/Engine.SpringArmComponent|GetTargetArmLength _springarm) 2e+02) 5e+03))))

(event Input|MouseEvents|MouseWheelUp
  (params (Key :type Key%20Structure :default "None"))
  (bind _springarm (Variables|Default|GetSpringArm))
  ;[1 1 1] Mouse View
  ;;[1 1 1] Збільшення коліщатка дальності камери
  (:Pressed
    (Variables|/Script/Engine.SpringArmComponent|SetTargetArmLength _springarm (Math|Float|Max(Float) (- (Variables|/Script/Engine.SpringArmComponent|GetTargetArmLength _springarm) 2e+02) 1e+02))))

(fn ConstructionScript)