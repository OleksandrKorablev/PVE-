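; Showcase Blueprint for the East T-72B tank that exposes its adjustable features to generic slider, button and checkbox input events.
; Each indexed event forwards its value to a setter for speed, skin, damage display, turret, gun, firing, hatches or light emissivity.
; The setters are not defined here, and the construction script only calls its parent.
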(event EventSetCheckboxVariable1
  (params (NewState :type Boolean))
  ;[1 1 1] Firing activation
  (CallFunction|SetFiring NewState))

(event EventSetSliderVariable6
  (params (NewValue :type Float%20%28double-precision%29))
  ;[1 1 1] Light emissivity
  (CallFunction|SetLightsEmissivity NewValue))

(event EventSetSliderVariable5
  (params (NewValue :type Float%20%28double-precision%29))
  ;[1 1 1] Command and Driver Hatch
  (CallFunction|SetHatchCommandAngle NewValue))

(event EventSetSliderVariable0
  (params (NewValue :type Float%20%28double-precision%29))
  ;[1 1 1] Speed
  (CallFunction|SetSpeed NewValue))

(event EventSetSliderVariable1
  (params (NewValue :type Float%20%28double-precision%29))
  ;[1 1 1] Turret rotation
  (CallFunction|SetTurretRotation NewValue))

(event EventSetSliderVariable2
  (params (NewValue :type Float%20%28double-precision%29))
  ;[1 1 1] Gun elevation
  (CallFunction|SetGunElevation NewValue))

(event EventSetSliderVariable3
  (params (NewValue :type Float%20%28double-precision%29))
  ;[1 1 1] Hatch angle
  (CallFunction|SetHatchesAngle NewValue))

(event EventSetSliderVariable4
  (params (NewValue :type Float%20%28double-precision%29))
  ;[1 1 1] Command and Driver Hatch
  (CallFunction|SetHatchDriverAngle NewValue))

(event EventSetButtonsVariable0
  (params (NewIndex :type Integer))
  ;[1 1 1] Skin variant
  (CallFunction|SetSkinType (Math|Conversions|ToFloat(Integer) NewIndex)))

(event EventSetCheckboxVariable0
  (params (NewState :type Boolean))
  ;[1 1 1] Show damage vehicle
  (CallFunction|SetShowDamage NewState))

(fn ConstructionScript
  (|CallParentFunction))